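; BP_CharacterStatusComponent is an actor component that stores and changes character status values, currently only Health.
; AddStatus and RemoveStatus switch on a status type and add or subtract the given amount through UpdateHealth.
; UpdateHealth clamps CurrentHealth between zero and MaxHealth, and GetStatusValue returns the current value for the requested status.
; It runs no event or tick logic, so values change only when these functions are called.
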(event EventBeginPlay)

(event EventTick
  (params (DeltaSeconds :type Float%20%28single-precision%29)))

(fn AddStatus
  (params (valueToAdd :type Float%20%28double-precision%29) (StatusToUpdate :type E_PawnStatus%20Enum :default "NewEnumerator0"))
  (LocalVariables|Set_valueToAdd valueToAdd)
  (switch Utilities|FlowControl|Switch|SwitchonE_PawnStatus StatusToUpdate
    (:NewEnumerator0
      (internal|UpdateHealth (+ (Variables|Default|GetCurrentHealth) valueToAdd)))))

(fn RemoveStatus
  (params (valueToRemove :type Float%20%28double-precision%29) (StatusToUpdate :type E_PawnStatus%20Enum :default "NewEnumerator0"))
  (LocalVariables|Set_valueToRemove valueToRemove)
  (switch Utilities|FlowControl|Switch|SwitchonE_PawnStatus StatusToUpdate
    (:NewEnumerator0
      (internal|UpdateHealth (- (Variables|Default|GetCurrentHealth) (LocalVariables|Get_valueToRemove))))))

(fn UpdateHealth
  (params (Value :type Float%20%28double-precision%29))
  (Variables|Default|SetCurrentHealth (Math|Float|Clamp(Float) Value 0.0 (Variables|Default|GetMaxHealth))))

(fn GetStatusValue
  (params (StatusToGet :type E_PawnStatus%20Enum :default "NewEnumerator0"))
  (switch Utilities|FlowControl|Switch|SwitchonE_PawnStatus StatusToGet
    (:NewEnumerator0
      (return (Variables|Default|GetCurrentHealth)))))