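; Actor component that runs replicated melee combat, telling normal from heavy attacks by how long the input is held.
; Initiate starts a server timer; consuming it early gives a normal attack, while holding past it gives a heavy one.
; The server multicasts the montage unless the mesh is already playing, with heavy attacks slower and dealing double damage.
; On montage notify, only the authority sphere-traces around the owner and applies damage.
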(event Custom|Multicast_ExecuteNormalAttack
  ;[1 1 1] Plays the attack montage for all players, but only triggers the collision check on the server
  (bind _notifyname (Animation|Montage|PlayMontage (Variables|Setup|GetOwnerSkeletalMeshComponent) "/Game/Characters/Barbarian/Animations/AM_Attack_Normal.AM_Attack_Normal")
    (:OnNotifyBegin
      (Networking|SwitchHasAuthority
        (:Authority
          (switch name _notifyname
            (:Notify_NormalAttack
              (CallFunction|ServerCheckifCausedDamage (Getters|GetFinalNormalAtttackDamage)))))))))

(event Custom|Server_ForceHeavyAttack
  (CallFunction|ServerAttackInput true)
  (Utilities|Time|ClearandInvalidateTimerbyHandle (Variables|Default|GetHeavyAttackTimerHandle)))

(event Custom|Server_CheckIfCausedDamage
  (params (BaseDamage :type Float%20%28single-precision%29))
  (bind _returnvalue (Components|GetOwner))
  (bind _returnvalue_2 (Transformation|GetActorLocation _returnvalue))
  ;[1 1 1] On Server, checks for collision and apply damage if possible
  (bind _outhit (Collision|SphereTraceByChannel _returnvalue_2 _returnvalue_2 1e+02 "TraceTypeQuery1" false 0 "None"))
  (Game|Damage|ApplyDamage (.hitactor _outhit) BaseDamage 0 0 "/Script/Engine.DamageType"))

(event Custom|Multicast_ExecuteHeavyAttack
  ;[1 1 1] Plays the attack montage for all players, but only triggers the collision check on the server
  ;;[1 0.455 0.4152] Slower animation
  (bind _notifyname (Animation|Montage|PlayMontage (Variables|Setup|GetOwnerSkeletalMeshComponent) "/Game/Characters/Barbarian/Animations/AM_Attack_Normal.AM_Attack_Normal" 0.5)
    (:OnNotifyBegin
      (Networking|SwitchHasAuthority
        (:Authority
          (switch name _notifyname
            (:Notify_NormalAttack
              (CallFunction|ServerCheckifCausedDamage (Getters|GetFinalHeavyAtttackDamage)))))))))

(event Custom|Server_ValidAttackTransactionConsume
  ;[1 0.6879 0.175] Prevents the Consume function to run even if re triggered by the owner after the heavy attak timer has elapsed
  (if (Utilities|Time|IsValidTimerHandle (Variables|Default|GetHeavyAttackTimerHandle))
    ;[1 1 1] If timer is active, then it is still a normal attack. Heavy attack otherwise
    (CallFunction|ServerAttackInput (not (Utilities|Time|IsTimerActivebyHandle (Variables|Default|GetHeavyAttackTimerHandle))))
    (Utilities|Time|ClearandInvalidateTimerbyHandle (Variables|Default|GetHeavyAttackTimerHandle))))

(event Custom|Server_AttackInput
  (params (IsHeavyAttack :type Boolean))
  ;[1 1 1] Asks the server to initiate the attack sequence
  ;;[1 0.6813 0.2921] Prevents the owner to attack if its already doing an animation (like attacking)
  (if (not (Audio|Components|Audio|IsPlaying (Variables|Setup|GetOwnerSkeletalMeshComponent)))
    (if IsHeavyAttack
      (CallFunction|MulticastExecuteHeavyAttack)
      (else
        (CallFunction|MulticastExecuteNormalAttack)))))

(event Custom|Server_ValidAttackTransactionInitiate
  (Utilities|Time|ClearandInvalidateTimerbyHandle (Variables|Default|GetHeavyAttackTimerHandle))
  (bind _returnvalue (Utilities|Time|SetTimerbyEvent (EventDispatchers|CreateEvent :!event Custom|Server_ForceHeavyAttack) (Variables|Config|GetHeavyAttackHoldDownTime)))
  (Variables|Default|SetHeavyAttackTimerHandle _returnvalue))

(event EventBeginPlay
  ;[1 1 1] If user didnt setup the skeletal mesh, then try to grab the first one from the actor owner
  (Utilities|IsValid (Variables|Setup|GetOwnerSkeletalMeshComponent)
    (:Is%20Not%20Valid
      (Variables|Setup|SetOwnerSkeletalMeshComponent (Actor|GetComponentbyClass (Components|GetOwner) "/Script/Engine.SkeletalMeshComponent")))))

(fn GetFinalNormalAtttackDamage
  (return (CallFunction|CalculateDamage)))

(fn CalculateDamage
  (return (LocalVariables|Get_arbitraryValueBasedOnWeapon)))

(fn InitiateAttackTransaction
  (CallFunction|ServerValidAttackTransactionInitiate))

(fn ConsumeAttackTransaction
  (CallFunction|ServerValidAttackTransactionConsume))

(fn ClearAttackTransaction)

(fn GetFinalHeavyAtttackDamage
  (return (* (CallFunction|CalculateDamage) 2.0)))

(fn SetupComponentReferences
  (params (OwnerSkeletalMeshComponent :type Skeletal%20Mesh%20Component%20Object%20Reference))
  (Variables|Setup|SetOwnerSkeletalMeshComponent OwnerSkeletalMeshComponent))