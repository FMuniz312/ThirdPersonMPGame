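; Lobby game mode that tracks connected player controllers and distributes session data to lobby clients.
; On login or logout it updates the player list, then after a short delay refreshes the lobby game state's PlayerState list.
; It then appends player names with a false flag to the session data, assigns each PlayerState a server order index and sends the data to each owning client.
; A helper caches the main menu HUD.
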(event EventBeginPlay)

(event EventTick
  (params (DeltaSeconds :type Float%20%28single-precision%29)))

(event EventOnLogout
  (params (ExitingController :type Controller%20Object%20Reference))
  (bind _asplayer_controller (Utilities|Casting|CastToPlayerController ExitingController))
  (Utilities|Array|RemoveItem (Variables|Default|GetAllPlayersInSession) _asplayer_controller)
  (Utilities|FlowControl|Delay 0.3)
  (CallFunction|UpdateSessionData))

(event EventPostLogin
  (params (NewPlayer :type Player%20Controller%20Object%20Reference))
  (bind _returnvalue (Utilities|Array|AddUnique (Variables|Default|GetAllPlayersInSession) NewPlayer))
  (if (> _returnvalue -1)
    (Utilities|FlowControl|Delay 0.3)
    (CallFunction|UpdateSessionData)))

(fn ConstructionScript)

(fn GetMainMenuHud
  (params (PlayerController :type Player%20Controller%20Object%20Reference))
  (bind _as_bp_main_menu_hud (Variables|Default|GetAs%20BP%20Main%20Menu%20HUD)
    (:then
      (return _as_bp_main_menu_hud))
    (:else
      (bind _asbp_main_menu_hud (Utilities|Casting|CastToBP_MainMenuHUD (HUD|GetHUD PlayerController)))
      (bind _output_get (Variables|Default|SetAs%20BP%20Main%20Menu%20HUD _asbp_main_menu_hud))
      (return _output_get))))

(fn UpdateSessionData
  (bind _asbp_lobby_game_state (Utilities|Casting|CastToBP_LobbyGameState (Game|GetGameState)))
  (Default|UpdatePlayerStatesList _asbp_lobby_game_state)
  (for _array_element (Variables|Default|GetAllPlayersInSession)
    (Utilities|Array|Add (LocalVariables|GetAllPlayersSessionData) (Utilities|Struct|MakePlayerSessionData (Utilities|String|StringToName (PlayerState|GetPlayerName (Variables|/Script/Engine.Controller|GetPlayerState _array_element))) false)))
  (for (_array_element_2 _array_index) (Variables|Default|GetAllPlayersInSession)
    (Variables|/Game/Core/Player/Lobby/BP_LobbyPlayerState.BP_LobbyPlayerState_C|SetPlayerServerOrderID (.AsBP%20Lobby%20Player%20State (Utilities|Casting|CastToBP_LobbyPlayerState (Variables|/Script/Engine.Controller|GetPlayerState _array_element_2))) _array_index)
    (Default|OwiningClientUpdateLobbyData (.AsBP%20Lobby%20Controller (Utilities|Casting|CastToBP_LobbyController _array_element_2)) (LocalVariables|GetAllPlayersSessionData))))