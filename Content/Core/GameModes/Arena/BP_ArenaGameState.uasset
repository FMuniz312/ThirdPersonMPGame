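; Arena game state that detects the end of a match and either restarts or closes it.
; A cached player count, despite its "alive" naming, tallies states flagged Dead; its RepNotify ends the match at one or fewer.
; Each player state gets a client finish call, and a one-shot server event starts a short timer.
; The timer server-travels back to Arena if multiple players remain, otherwise destroys the session and opens the main menu.
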(event Custom|Server_FinishMatch
  (Utilities|FlowControl|DoOnce false
    (:Completed
      (bind _returnvalue (Utilities|Time|SetTimerbyEvent (delegate Custom|Server_FinishingMatch) 3.0))
      (Variables|Default|SetEndingMatchCountDown _returnvalue))))

(event Custom|Server_FinishingMatch
  (if (CallFunction|AreThereStillOtherPlayersintheGame)
    ;[1 1 1] HardReset
    (Development|ExecuteConsoleCommand "servertravel Arena?Listen" (Game|GetPlayerController 0))
    (else
      ;[1 1 1] Back to menu
      (|DestroySession (Game|GetPlayerController 0)
        (:OnSuccess
          _)
        (:OnFailure
          _))
      (Game|OpenLevel(byObjectReference) "/Game/Maps/MainMenu.MainMenu"))))

(fn ConstructionScript)

(fn AmountOfPlayersAlive
  (LocalVariables|Set_numberOfAlivePlayers 0)
  (for _array_element (Variables|Default|GetPlayerArray)
    (bind _asbp_player_state_arena (Utilities|Casting|CastToBP_PlayerState_Arena _array_element))
    (if (Variables|/Game/Core/Player/Arena/BP_PlayerState_Arena.BP_PlayerState_Arena_C|GetDead _asbp_player_state_arena)
      (LocalVariables|Set_numberOfAlivePlayers (+ (LocalVariables|Get_numberOfAlivePlayers) 1))))
  (return (LocalVariables|Get_numberOfAlivePlayers)))

(fn UpdateNumberOfPlayersALiveCache
  (Variables|Default|SetNumberOfPlayersAllive (CallFunction|AmountOfPlayersAlive)))

(fn OnRepNumberOfPlayersAllive
  (if (<= (Variables|Default|GetNumberOfPlayersAllive) 1)
    (for _array_element (Variables|Default|GetPlayerArray)
      (bind _asbp_player_state_arena (Utilities|Casting|CastToBP_PlayerState_Arena _array_element))
      (Default|ClientFinishMatch _asbp_player_state_arena))
    (CallFunction|ServerFinishMatch)))

(fn AreThereStillOtherPlayersintheGame
  (return (> (Utilities|Array|Length (Variables|Default|GetPlayerArray)) 1)))