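; Light normal-attack gameplay ability that overrides only the damage step, leaving its event graph as unused stubs.
; ApplyDamage picks a shield or normal damage effect depending on whether the target has the Block tag.
; It passes the owner combat component's negated final light-attack damage as a SetByCaller magnitude and applies the spec to the target.
; The target's combat component then multicasts the light damage GameplayCue, blocked or not.
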(event Ability|EventActivateAbility
  (|CallParentFunction) ; This node is disabled and will not be called.\nDrag off pins to build functionality.
)

(event Ability|EventOnEndAbility
  (params (bWasCancelled :type Boolean)))

(fn ApplyDamage
  (Utilities|IsValid (Variables|Default|GetCurrentTargetsAbillitySystem)
    (:Is%20Valid
      (bind _output_get (LocalVariables|Set_targetIsBlocking (GameplayTags|HasMatchingGameplayTag (Variables|Default|GetCurrentTargetsAbillitySystem) "(TagName=\"GameplayStatus.Character.Block\")")))
      (LocalVariables|SetcurrentEffectSpec (Ability|MakeOutgoingGameplayEffectSpec (select _output_get "/Game/Core/GAS/BP_ShieldDamageGameplayEffect_Light.BP_ShieldDamageGameplayEffect_Light_C" "/Game/Core/GAS/BP_NormalDamageGameplayEffect_Light.BP_NormalDamageGameplayEffect_Light_C")))
      (Ability|GameplayEffect|AssignTagSetbyCallerMagnitude (LocalVariables|GetcurrentEffectSpec) (LocalVariables|GetAttackTag) (* (Default|GetFinalLightAtttackDamage (Actor|GetComponentbyClass (Variables|Default|GetCharacterOwner) "/Game/Core/Combat/BP_CombatComponent.BP_CombatComponent_C")) -1.0))
      (GameplayEffects|ApplyGameplayEffectSpecToTarget (Variables|Default|GetownerAbilitySystem) (LocalVariables|GetcurrentEffectSpec) (Variables|Default|GetCurrentTargetsAbillitySystem))
      (Default|MulticastGameplayCueReplication (Actor|GetComponentbyClass (Components|GetOwner (Variables|Default|GetCurrentTargetsAbillitySystem)) "/Game/Core/Combat/BP_CombatComponent.BP_CombatComponent_C") "(TagName=\"GameplayCue.Damage.Normal.Light\")"))))