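; Heavy variant of the normal attack gameplay ability that supplies its own ApplyDamage logic.
; It checks the target's ability system for active Block effects to choose between the heavy shield damage and heavy normal damage GameplayEffects.
; The owner's combat component supplies the final heavy damage, passed negated as a SetByCaller magnitude under the heavy attack tag, and the spec is applied to the target.
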(event Ability|EventActivateAbility
  (|CallParentFunction) ; This node is disabled and will not be called.\nDrag off pins to build functionality.
)

(event Ability|EventOnEndAbility
  (params (bWasCancelled :type Boolean)))

(fn ApplyDamage
  (Utilities|IsValid (Variables|Default|GetCurrentTargetsAbillitySystem)
    (:Is%20Valid
      (bind _returnvalue (GameplayEffects|GetActiveEffectswithAllTags (Variables|Default|GetCurrentTargetsAbillitySystem) "(GameplayTags=((TagName=\"GameplayAbility.Combat.Defense.Block\")))"))
      (bind _output_get (LocalVariables|Set_targetIsBlocking (Utilities|Array|IsNotEmpty _returnvalue)))
      (LocalVariables|SetcurrentEffectSpec (Ability|MakeOutgoingGameplayEffectSpec (select _output_get "/Game/Core/GAS/BP_ShieldDamageGameplayEffect_Heavy.BP_ShieldDamageGameplayEffect_Heavy_C" "/Game/Core/GAS/BP_NormalDamageGameplayEffect_Heavy.BP_NormalDamageGameplayEffect_Heavy_C")))
      (Ability|GameplayEffect|AssignTagSetbyCallerMagnitude (LocalVariables|GetcurrentEffectSpec) "(TagName=\"GameplayAbility.Combat.Attack.Heavy\")" (* (Default|GetFinalHeavyAtttackDamage (Actor|GetComponentbyClass (Variables|Default|GetCharacterOwner) "/Game/Core/Combat/BP_CombatComponent.BP_CombatComponent_C")) -1.0))
      (GameplayEffects|ApplyGameplayEffectSpecToTarget (Variables|Default|GetownerAbilitySystem) (LocalVariables|GetcurrentEffectSpec) (Variables|Default|GetCurrentTargetsAbillitySystem)))))