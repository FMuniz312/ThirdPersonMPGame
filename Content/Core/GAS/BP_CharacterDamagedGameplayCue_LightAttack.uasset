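; Gameplay Cue actor that plays hit feedback when a character takes light-attack damage.
; On execute, it casts its owner to Character and spawns a pooled light damage-burst Niagara effect at that location.
; Locally controlled characters also get a world camera shake, while other clients only print a placeholder debug string.
; A non-character owner gets just a debug print.
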(event EventBeginPlay)

(event Collision|EventActorBeginOverlap
  (params (OtherActor :type Actor%20Object%20Reference)))

(event EventTick
  (params (DeltaSeconds :type Float%20%28single-precision%29)))

(fn ConstructionScript)

(fn OnExecute
  (params (MyTarget :type Actor%20Object%20Reference) (Parameters :type Gameplay%20Cue%20Parameters%20Structure%20%28by%20ref%29))
  (bind _ascharacter (Utilities|Casting|CastToCharacter (Components|GetOwner))
    (:then
      (Niagara|SpawnSystematLocation (Components|GetOwner) "/Game/Effects/Combat/NS_DamageBurst_Light.NS_DamageBurst_Light" (Transformation|GetActorLocation (Components|GetOwner)) "0, 0, 0" "1.000000,1.000000,1.000000" true true "AutoRelease")
      (if (Pawn|IsLocallyControlled _ascharacter)
        ;[0.96 1 0.3012] Owner Only Effects
        (Camera|PlayWorldCameraShake (Components|GetOwner) "/Game/Effects/Combat/BP_NormalDamageCameraShake_Light.BP_NormalDamageCameraShake_Light_C" (Transformation|GetActorLocation (Components|GetOwner)) 5e+03 5e+03)
        (return true)
        (else
          (Development|PrintString (Components|GetOwner) "Everyone elses effects")
          (return true))))
    (:CastFailed
      (Development|PrintString (Components|GetOwner) "Damage was dealt")
      (return true))))