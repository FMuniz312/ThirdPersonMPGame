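; Gameplay Ability for a normal melee attack that finds pawns in front of the owning character.
; On activation it runs a zero-length sphere trace a short distance ahead, ignoring the owner, and caches each hit actor's Ability System Component.
; It calls ApplyDamage for each valid component, then ends the ability.
; ApplyDamage is empty here, so this Blueprint itself deals no damage.
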(event Ability|EventActivateAbility
  (bind _output_get (Variables|Default|SetCharacterOwner (Ability|GetOwningActorfromActorInfo)))
  (Variables|Default|SetownerAbilitySystem (Ability|GetAbilitySystemComponent _output_get))
  (bind _outhits (Collision|MultiSphereTraceForObjects (+ (Transformation|GetActorLocation (Variables|Default|GetCharacterOwner)) (* (Transformation|GetActorForwardVector (Variables|Default|GetCharacterOwner)) 1e+02)) (+ (Transformation|GetActorLocation (Variables|Default|GetCharacterOwner)) (* (Transformation|GetActorForwardVector (Variables|Default|GetCharacterOwner)) 1e+02)) 7e+01 (Utilities|Array|MakeArray "ObjectTypeQuery3") false (Utilities|Array|MakeArray (Variables|Default|GetCharacterOwner)) "None"))
  (for _array_element _outhits
    (bind _output_get_2 (Variables|Default|SetCurrentTargetsAbillitySystem (Ability|GetAbilitySystemComponent (.hitactor _array_element))))
    (Utilities|IsValid _output_get_2
      (:Is%20Valid
        (CallFunction|ApplyDamage))))
  (Variables|Default|SetCurrentTargetsAbillitySystem 0)
  (Ability|EndAbility))

(fn ApplyDamage)