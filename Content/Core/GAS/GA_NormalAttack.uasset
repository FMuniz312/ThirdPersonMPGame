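; Gameplay ability for a normal light attack that damages pawns just in front of the owner.
; On activation, a stationary multi-sphere trace ahead of the owner, with debug drawing, finds targets with an Ability System Component, then the ability ends.
; Each target applies GE_NormalDamage_Light to itself, and the active effect's SetByCaller magnitude is updated afterward with the light attack damage from the owner's BP_CombatComponent.
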(event Ability|EventActivateAbility
  (Variables|Default|SetCharacterOwner (Ability|GetOwningActorfromActorInfo))
  (bind _outhits (Collision|MultiSphereTraceForObjects (+ (Transformation|GetActorLocation (Variables|Default|GetCharacterOwner)) (* (Transformation|GetActorForwardVector (Variables|Default|GetCharacterOwner)) 1e+02)) (+ (Transformation|GetActorLocation (Variables|Default|GetCharacterOwner)) (* (Transformation|GetActorForwardVector (Variables|Default|GetCharacterOwner)) 1e+02)) 7e+01 (Utilities|Array|MakeArray "ObjectTypeQuery3") false (Utilities|Array|MakeArray (Variables|Default|GetCharacterOwner)) "ForDuration"))
  (for _array_element _outhits
    (bind _output_get (Variables|Default|SetCurrentTargetsAbillitySystem (Ability|GetAbilitySystemComponent (.hitactor _array_element))))
    (Utilities|IsValid _output_get
      (:Is%20Valid
        (CallFunction|ApplyDamage))))
  (Ability|EndAbility))

(fn ApplyDamage
  (bind _currenttargetsabillitysystem (Variables|Default|GetCurrentTargetsAbillitySystem))
  (bind _returnvalue (GameplayEffects|ApplyGameplayEffectToSelf :self _currenttargetsabillitysystem :GameplayEffectClass "/Game/Core/GAS/GE_NormalDamage_Light.GE_NormalDamage_Light_C"))
  (Class|AbilitySystemComponent|UpdateActiveGameplayEffectSetbyCallerMagnitude _currenttargetsabillitysystem _returnvalue "(TagName=\"GameplayAbility.Combat.Attack.Light\")" (Default|GetFinalLightAtttackDamage (Actor|GetComponentbyClass (Variables|Default|GetCharacterOwner) "/Game/Core/Combat/BP_CombatComponent.BP_CombatComponent_C"))))