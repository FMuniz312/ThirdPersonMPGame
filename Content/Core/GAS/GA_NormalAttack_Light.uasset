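; Gameplay Ability for a character's light normal attack, defining how it damages the current target.
; ApplyDamage checks the target's Ability System for the Block tag to choose between light shield damage and normal damage effects.
; It sets the effect's magnitude by caller tag to the negated final light attack damage from the owner's combat component, then applies it to the target.
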(event Ability|EventActivateAbility
  (|CallParentFunction) ; This node is disabled and will not be called.\nDrag off pins to build functionality.
)

(event Ability|EventOnEndAbility
  (params (bWasCancelled :type Boolean)))

(fn ApplyDamage
  (Utilities|IsValid (Variables|Default|GetCurrentTargetsAbillitySystem)
    (:Is%20Valid
      (bind _output_get (LocalVariables|Set_targetIsBlocking (GameplayTags|HasMatchingGameplayTag (Variables|Default|GetCurrentTargetsAbillitySystem) "(TagName=\"GameplayStatus.Character.Block\")")))
      (LocalVariables|SetcurrentEffectSpec (Ability|MakeOutgoingGameplayEffectSpec (select _output_get "/Game/Core/GAS/GE_ShieldDamage_Light.GE_ShieldDamage_Light_C" "/Game/Core/GAS/GE_NormalDamage_Light.GE_NormalDamage_Light_C")))
      (Ability|GameplayEffect|AssignTagSetbyCallerMagnitude (LocalVariables|GetcurrentEffectSpec) "(TagName=\"GameplayAbility.Combat.Attack.Light\")" (* (Default|GetFinalLightAtttackDamage (Actor|GetComponentbyClass (Variables|Default|GetCharacterOwner) "/Game/Core/Combat/BP_CombatComponent.BP_CombatComponent_C")) -1.0))
      (GameplayEffects|ApplyGameplayEffectSpecToTarget (Variables|Default|GetownerAbilitySystem) (LocalVariables|GetcurrentEffectSpec) (Variables|Default|GetCurrentTargetsAbillitySystem)))))