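; Character status component that applies stun and death to its owning character, with its listeners running on the server.
; Stun tag queries zero walk speeds and disable movement, then restore cached defaults via Falling mode.
; When a watched attribute drops to zero or below, it destroys the owner.
; As an acknowledged replication workaround, it also flags the arena PlayerState dead and refreshes the GameState's alive-player count.
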(event EventBeginPlay
  (Networking|SwitchHasAuthority
    (:Authority
      (Utilities|FlowControl|Sequence
        (:then_0
          (Ability|Tasks|WaitGameplayTagQueryOnActor (Components|GetOwner) "(TokenStreamVersion=0,TagDictionary=((TagName=\"GameplayStatus.Character.Stun\")),QueryTokenStream=(0,1,2,1,0),UserDescription=\"Is Stunned\",AutoDescription=\" ALL( GameplayStatus.Character.Stun )\")"
            (:Triggered
              (CallFunction|ApplyStun))))
        (:then_1
          (Ability|Tasks|WaitGameplayTagQueryOnActor (Components|GetOwner) "(TokenStreamVersion=0,TagDictionary=((TagName=\"GameplayStatus.Character.Stun\")),QueryTokenStream=(0,1,2,1,0),UserDescription=\"Is Stunned\",AutoDescription=\" ALL( GameplayStatus.Character.Stun )\")" "WhenFalse"
            (:Triggered
              (CallFunction|RemoveStun))))
        (:then_2
          (bind _newvalue (Ability|Tasks|WaitForAttributeChanged (Components|GetOwner) "(AttributeName=\"Health\",Attribute=/Script/ThirdPersonMPGame.GameAttributeSet:Health,AttributeOwner=\"/Script/CoreUObject.Class'/Script/ThirdPersonMPGame.GameAttributeSet'\")")
            (:Changed
              ;[1 0.0828 0.1126] bye bye me
              (if (<= _newvalue 0.0)
                (Development|PrintString "im dead")
                (Networking|SwitchHasAuthority
                  (:Authority
                    (Utilities|FlowControl|Sequence
                      (:then_0
                        ;[1 0.09896 0.09896] Not in the right place, but I had to leave it here to fix a replication issue that I didnt have time to properly change
                        (bind _ascharacter (Utilities|Casting|CastToCharacter (Components|GetOwner)))
                        (bind _asbp_player_state_arena (Utilities|Casting|CastToBP_PlayerState_Arena (Variables|/Script/Engine.Pawn|GetPlayerState _ascharacter)))
                        (Variables|/Game/Core/Player/Arena/BP_PlayerState_Arena.BP_PlayerState_Arena_C|SetDead _asbp_player_state_arena true)
                        (bind _asbp_arena_game_state (Utilities|Casting|CastToBP_ArenaGameState (Game|GetGameState)))
                        (Default|UpdateNumberOfPlayersALiveCache _asbp_arena_game_state))
                      (:then_1
                        (Actor|DestroyActor (Components|GetOwner))))))))))))))

(fn GetCharacterMovementComponent
  (Utilities|IsValid (Variables|Default|GetownerCharacterMovementComponent)
    (:Is%20Valid
      (return (Variables|Default|GetownerCharacterMovementComponent)))
    (:Is%20Not%20Valid
      (bind _output_get (Variables|Default|SetownerCharacterMovementComponent (Actor|GetComponentbyClass (Components|GetOwner) "/Script/Engine.CharacterMovementComponent")))
      (Variables|Setup|SetDefaultMaxSpeed (Variables|/Script/Engine.CharacterMovementComponent|GetMaxWalkSpeed _output_get))
      (Variables|Setup|SetDefaultMaxCrouchSpeed (Variables|/Script/Engine.CharacterMovementComponent|GetMaxWalkSpeedCrouched _output_get))
      (return _output_get))))

(fn ApplyStun
  (Variables|/Script/Engine.CharacterMovementComponent|SetMaxWalkSpeed (Getter|GetCharacterMovementComponent) 0.0)
  (Variables|/Script/Engine.CharacterMovementComponent|SetMaxWalkSpeedCrouched (Getter|GetCharacterMovementComponent) 0.0)
  (Components|Movement|StopMovementImmediately (Getter|GetCharacterMovementComponent))
  (Pawn|Components|CharacterMovement|SetMovementMode (Getter|GetCharacterMovementComponent) "MOVE_None" 0))

(fn RemoveStun
  (Variables|/Script/Engine.CharacterMovementComponent|SetMaxWalkSpeed (Getter|GetCharacterMovementComponent) (Variables|Setup|GetDefaultMaxSpeed))
  (Variables|/Script/Engine.CharacterMovementComponent|SetMaxWalkSpeedCrouched (Getter|GetCharacterMovementComponent) (Variables|Setup|GetDefaultMaxCrouchSpeed))
  ;[1 1 1] Unreal character base class automatically checks if its grounded to then set it to Walking mode
  (Pawn|Components|CharacterMovement|SetMovementMode (Getter|GetCharacterMovementComponent) "MOVE_Falling" 0))