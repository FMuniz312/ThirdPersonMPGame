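; Combat component that grants light and heavy Gameplay Ability System attacks to its owner and handles their replicated execution.
; A server timer turns press and release into a light attack, or a forced heavy one when held long enough.
; Multicasts play one montage, slower for heavy, lock re-attacks, and activate the tagged ability only on authority at the notify.
; Blocking-tag waits, movement-speed helpers and weapon damage are unfinished stubs.
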(event EventBeginPlay
  (Setup|SetupAbilitySystemDependency)
  (CallFunction|BeginPlayDefensiveGraph))

(event Custom|Multicast_ExecuteLightAttack
  ;[1 1 1] Plays the attack montage for all players, but only triggers the collision check on the server
  (bind _notifyname (Animation|Montage|PlayMontage (Getters|GetOwnerSkeletalMesh) "/Game/Characters/Barbarian/Animations/AM_Attack_Normal.AM_Attack_Normal")
    (:then
      (Control|LockAttack))
    (:OnCompleted
      (Control|UnlockAttack :!label _label))
    (:OnInterrupted
      (goto _label))
    (:OnNotifyBegin
      (Networking|SwitchHasAuthority
        (:Authority
          (switch name _notifyname
            (:Notify_NormalAttack
              (Abilities|TryActivateAbilitiesbyTag (Variables|Components|GetOwnerAbilitySystem) (GameplayTags|MakeGameplayTagContainerfromTag "(TagName=\"GameplayAbility.Combat.Attack.Light\")") false))))))))

(event Custom|Server_ForceHeavyAttack
  (CallFunction|ServerAttackInput true)
  (Utilities|Time|ClearandInvalidateTimerbyHandle (Variables|Default|GetHeavyAttackTimerHandle)))

(event Custom|Multicast_ExecuteHeavyAttack
  ;[1 1 1] Plays the attack montage for all players, but only triggers the collision check on the server
  ;;[1 0.455 0.4152] Slower animation
  (bind _notifyname (Animation|Montage|PlayMontage (Getters|GetOwnerSkeletalMesh) "/Game/Characters/Barbarian/Animations/AM_Attack_Normal.AM_Attack_Normal" 0.5)
    (:then
      (Control|LockAttack))
    (:OnCompleted
      (Control|UnlockAttack :!label _label))
    (:OnInterrupted
      (goto _label))
    (:OnNotifyBegin
      (Networking|SwitchHasAuthority
        (:Authority
          (switch name _notifyname
            (:Notify_NormalAttack
              (Abilities|TryActivateAbilitiesbyTag (Variables|Components|GetOwnerAbilitySystem) (GameplayTags|MakeGameplayTagContainerfromTag "(TagName=\"GameplayAbility.Combat.Attack.Heavy\")") false))))))))

(event Custom|Server_ValidAttackTransactionConsume
  ;[1 0.6879 0.175] Prevents the Consume function to run even if re triggered by the owner after the heavy attak timer has elapsed
  (if (Utilities|Time|IsValidTimerHandle (Variables|Default|GetHeavyAttackTimerHandle))
    ;[1 1 1] If timer is active, then it is still a normal attack. Heavy attack otherwise
    (CallFunction|ServerAttackInput (not (Utilities|Time|IsTimerActivebyHandle (Variables|Default|GetHeavyAttackTimerHandle))))
    (Utilities|Time|ClearandInvalidateTimerbyHandle (Variables|Default|GetHeavyAttackTimerHandle))))

(event Custom|Server_AttackInput
  (params (IsHeavyAttack :type Boolean))
  ;[1 1 1] Asks the server to initiate the attack sequence
  ;;[1 0.6813 0.2921] Prevents the owner to attack if its already attacking
  (if (not (Variables|Default|GetCurrentlyAttacking))
    (if IsHeavyAttack
      (CallFunction|MulticastExecuteHeavyAttack)
      (else
        (CallFunction|MulticastExecuteLightAttack)))))

(event Custom|Server_ValidAttackTransactionInitiate
  (Utilities|Time|ClearandInvalidateTimerbyHandle (Variables|Default|GetHeavyAttackTimerHandle))
  (bind _returnvalue (Utilities|Time|SetTimerbyEvent (EventDispatchers|CreateEvent :!event Custom|Server_ForceHeavyAttack) (Variables|Config|GetHeavyAttackHoldDownTime)))
  (Variables|Default|SetHeavyAttackTimerHandle _returnvalue))

(event Custom|BeginPlay_DefensiveGraph
  (Networking|SwitchHasAuthority
    (:Authority
      (Utilities|FlowControl|Sequence
        (:then_0
          (Ability|Tasks|WaitGameplayTagQueryOnActor (Components|GetOwner) (Variables|Default|GetIsBlockingTagQuery)))
        (:then_1
          (Ability|Tasks|WaitGameplayTagQueryOnActor (Components|GetOwner) (Variables|Default|GetIsBlockingTagQuery) "WhenFalse"))))))

(fn GetFinalLightAtttackDamage
  (return (Setup|CalculateDamage)))

(fn CalculateDamage
  (return (LocalVariables|Get_arbitraryValueBasedOnWeapon)))

(fn InitiateAttackTransaction
  (CallFunction|ServerValidAttackTransactionInitiate))

(fn ConsumeAttackTransaction
  (CallFunction|ServerValidAttackTransactionConsume))

(fn ClearAttackTransaction)

(fn GetFinalHeavyAtttackDamage
  (return (* (Setup|CalculateDamage) 2.0)))

(fn SetupComponentReferences
  (params (OwnerSkeletalMeshComponent :type Skeletal%20Mesh%20Component%20Object%20Reference))
  (Variables|Components|SetOwnerSkeletalMeshComponent OwnerSkeletalMeshComponent))

(fn SetupAbilitySystemDependency
  (GameplayAbilities|GiveAbility (Getters|GetOwnerAbilitySystem) "/Game/Core/GAS/GA_NormalAttack_Light.GA_NormalAttack_Light_C" 0 -1)
  (GameplayAbilities|GiveAbility (Getters|GetOwnerAbilitySystem) "/Game/Core/GAS/GA_NormalAttack_Heavy.GA_NormalAttack_Heavy_C" 0 -1))

(fn LockAttack
  (Variables|Default|SetCurrentlyAttacking true))

(fn UnlockAttack
  (Variables|Default|SetCurrentlyAttacking false))

(fn GetOwnerSkeletalMesh
  (Utilities|IsValid (Variables|Components|GetOwnerSkeletalMeshComponent)
    (:Is%20Valid
      _)
    (:Is%20Not%20Valid
      (Variables|Components|SetOwnerSkeletalMeshComponent (Actor|GetComponentbyClass (Components|GetOwner) "/Script/Engine.SkeletalMeshComponent"))))
  (return (Variables|Components|GetOwnerSkeletalMeshComponent)))

(fn GetOwnerAbilitySystem
  (Utilities|IsValid (Variables|Components|GetOwnerAbilitySystem)
    (:Is%20Valid
      _)
    (:Is%20Not%20Valid
      (Variables|Components|SetOwnerAbilitySystem (Actor|GetComponentbyClass (Components|GetOwner) "/Script/GameplayAbilities.AbilitySystemComponent"))))
  (return (Variables|Components|GetOwnerAbilitySystem)))

(fn GetCharacterMovementComponent
  (return 0))

(fn SlowCharacterDown
  (Variables|/Script/Engine.CharacterMovementComponent|SetMaxWalkSpeed (CallFunction|GetCharacterMovementComponent) 0.0)
  (Variables|/Script/Engine.CharacterMovementComponent|SetMaxWalkSpeedCrouched (CallFunction|GetCharacterMovementComponent) 0.0))

(fn ResetCharacterSpeed
  (Variables|/Script/Engine.CharacterMovementComponent|SetMaxWalkSpeed (CallFunction|GetCharacterMovementComponent) 0.0)
  (Variables|/Script/Engine.CharacterMovementComponent|SetMaxWalkSpeedCrouched (CallFunction|GetCharacterMovementComponent) 0.0))