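; Player state for Arena matches that shows the end-of-game screen and keeps its countdown current.
; Client_FinishMatch waits briefly, then creates WBP_EndGame_Screen, marking the player as winner if not Dead, and adds it to the player screen.
; Tick copies the remaining time of the game state's EndingMatchCountDown timer into that widget as whole seconds.
; A helper lazily casts and caches the BP_ArenaGameState reference.
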(event Custom|Client_FinishMatch
  (Utilities|FlowControl|Delay 1.0)
  (bind _returnvalue (UserInterface|CreateWidget "/Game/UI/EndGame/WBP_EndGame_Screen.WBP_EndGame_Screen_C"))
  (Variables|Default|SetWBP_EndGameScreen _returnvalue)
  (Variables|/Game/UI/EndGame/WBP_EndGame_Screen.WBP_EndGame_Screen_C|SetbHasWon (Variables|Default|GetWBP_EndGameScreen) (not (Variables|Default|GetDead)))
  (UserInterface|Viewport|AddtoPlayerScreen (Variables|Default|GetWBP_EndGameScreen)))

(event EventBeginPlay)

(event EventTick
  (params (DeltaSeconds :type Float%20%28single-precision%29))
  (if (Utilities|Time|IsValidTimerHandle (Variables|/Game/Core/GameModes/Arena/BP_ArenaGameState.BP_ArenaGameState_C|GetEndingMatchCountDown (CallFunction|GetArenaGameState)))
    (bind _wbp_endgamescreen (Variables|Default|GetWBP_EndGameScreen)
      (:then
        (Variables|/Game/UI/EndGame/WBP_EndGame_Screen.WBP_EndGame_Screen_C|SetCurrentCountdown _wbp_endgamescreen (Math|Float|Truncate (Utilities|Time|GetTimerRemainingTimebyHandle (Variables|/Game/Core/GameModes/Arena/BP_ArenaGameState.BP_ArenaGameState_C|GetEndingMatchCountDown (CallFunction|GetArenaGameState))))))
      (:else))))

(fn ConstructionScript)

(fn GetArenaGameState
  (bind _as_bp_arena_game_state (Variables|Default|GetAs%20BP%20Arena%20Game%20State)
    (:then
      (return _as_bp_arena_game_state))
    (:else
      (bind _asbp_arena_game_state (Utilities|Casting|CastToBP_ArenaGameState (Game|GetGameState)))
      (bind _output_get (Variables|Default|SetAs%20BP%20Arena%20Game%20State _asbp_arena_game_state))
      (return _output_get))))