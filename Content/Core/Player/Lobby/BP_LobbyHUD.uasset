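; BP_LobbyHUD is the lobby HUD that shows the room screen and passes player state to it.
; On BeginPlay it creates WBP_LobbyRoom_Screen, adds it to the player screen, and switches to UI-only input with a visible cursor.
; Client_UpdateLobbyPlayers forwards all player states to that widget, reopening the lobby first if the widget is invalid.
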(event Custom|Client_UpdateLobbyPlayers
  (params (AllPlayersState :type Array%20of%20Player%20Session%20Data%20Structures))
  (bind _wbp_lobbyroom (Variables|Default|GetWBP_LobbyRoom)
    (:then
      _)
    (:else
      (CallFunction|ClientOpenLobby)))
  (Default|UpdateLobbyPlayersData _wbp_lobbyroom AllPlayersState))

(event Custom|Client_OpenLobby
  (bind _returnvalue (UserInterface|CreateWidget "/Game/UI/Lobby/WBP_LobbyRoom_Screen.WBP_LobbyRoom_Screen_C"))
  (bind _output_get (Variables|Default|SetWBP_LobbyRoom _returnvalue))
  (UserInterface|Viewport|AddtoPlayerScreen _output_get 100))

(event EventBeginPlay
  (bind _returnvalue (Game|GetPlayerController 0))
  (CallFunction|ClientOpenLobby)
  (Input|SetInputModeUIOnly _returnvalue 0 "DoNotLock" false)
  (Variables|/Script/Engine.PlayerController|SetbShowMouseCursor _returnvalue true))

(fn ConstructionScript)